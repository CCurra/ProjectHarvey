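; LevelLoader is an actor that moves the player on to the next level in TreasureHunter when the player character overlaps it.
; On BeginPlay it turns off collision on its Cube, toggles that mesh's visibility, and switches on the current level name to choose a hard-coded successor, with Tombs leading to End.
; Its overlap event opens that stored level by name, ignoring actors other than the player character.
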(event EventBeginPlay
  (Collision|SetCollisionEnabled (Variables|Default|GetCube) "NoCollision")
  (Rendering|ToggleVisibility (Variables|Default|GetCube) false)
  (bind _returnvalue (Game|GetCurrentLevelName true))
  (bind _output_get (Variables|Default|SetCurrentLevel (Utilities|String|StringToName _returnvalue)))
  (switch name _output_get
    (:Beach
      (Variables|Default|SetNextLevel (Variables|Default|GetLevel2)))
    (:Jungle
      (Variables|Default|SetNextLevel (Variables|Default|GetLevel3)))
    (:cliff
      (Variables|Default|SetNextLevel (Variables|Default|GetLevel4)))
    (:Tombs
      (Variables|Default|SetNextLevel (Variables|Default|GetEnd)))))

(event Collision|EventActorBeginOverlap
  (params (OtherActor :type Actor%20Object%20Reference))
  (if (== OtherActor (Game|GetPlayerCharacter 0))
    (Game|OpenLevel(byName) (Variables|Default|GetNextLevel))))

(event EventTick
  (params (DeltaSeconds :type Float%20%28single-precision%29)))

(fn ConstructionScript)