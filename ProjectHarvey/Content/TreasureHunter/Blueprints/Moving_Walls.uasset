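; Moving walls actor for TreasureHunter that slides two cube meshes toward target positions once an actor overlaps it.
; BeginPlay hides the two MoveTo markers and disables their collision.
; Overlap by any actor sets a flag (the player check is unwired), and Tick then eases each cube's relative location toward its marker by lerping with DeltaSeconds times Timer, without sweep.
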(event EventBeginPlay
  (Rendering|SetVisibility (Variables|Default|GetMoveTo2) false false)
  (Rendering|SetVisibility (Variables|Default|GetMoveTo1) false false)
  (Collision|SetCollisionEnabled (Variables|Default|GetMoveTo1) "NoCollision")
  (Collision|SetCollisionEnabled (Variables|Default|GetMoveTo2) "NoCollision"))

(event Collision|EventActorBeginOverlap
  (params (OtherActor :type Actor%20Object%20Reference))
  (Variables|Default|SetName true))

(event EventTick
  (params (DeltaSeconds :type Float%20%28single-precision%29))
  (bind _timer (Variables|Default|GetTimer))
  (bind _returnvalue (* DeltaSeconds _timer))
  (if (Variables|Default|GetName)
    (Transformation|SetRelativeLocation (Variables|Default|GetCube1) (.Location (Math|Transform|BreakTransform (Math|Transform|Lerp(Transform) (Transformation|GetRelativeTransform (Variables|Default|GetCube1)) (Transformation|GetRelativeTransform (Variables|Default|GetMoveTo1)) _returnvalue))) false false)
    (Transformation|SetRelativeLocation (Variables|Default|GetCube2) (.Location (Math|Transform|BreakTransform (Math|Transform|Lerp(Transform) (Transformation|GetRelativeTransform (Variables|Default|GetCube2)) (Transformation|GetRelativeTransform (Variables|Default|GetMoveTo2)) _returnvalue))) false false)))

(fn ConstructionScript)