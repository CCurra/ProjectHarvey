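; EnemyRunner is an enemy that idles until the player overlaps it, then runs at them and explodes on reaching them.
; While overlapping, Tick yaws it toward the player and lerps its location closer by delta time, without sweep.
; Within a set distance it makes the SceneManager, fetched from the player character at BeginPlay, deduct HP as "SpearIslander", then plays a groan and explosion and destroys itself.
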(event Collision|EventActorBeginOverlap
  (params (OtherActor :type Actor%20Object%20Reference))
  (bind _returnvalue (Game|GetPlayerCharacter 0))
  (if (== OtherActor _returnvalue)
    (Variables|Default|SetThirdPersonCharacter _returnvalue)
    (Variables|Default|SetOverlappingCharacter true)
    (Components|Animation|PlayAnimation (Variables|Character|GetMesh) "/Game/Character/MaleIslander1/Animations/ThirdPersonRun.ThirdPersonRun" true)))

(event Collision|EventActorEndOverlap
  (params (OtherActor :type Actor%20Object%20Reference))
  (if (== OtherActor (Game|GetPlayerCharacter 0))
    (Variables|Default|SetOverlappingCharacter false)
    (Components|Animation|PlayAnimation (Variables|Character|GetMesh) "/Game/Character/MaleIslander1/Animations/ThirdPersonIdle.ThirdPersonIdle" true)))

(event EventTick
  (params (DeltaSeconds :type Float%20%28single-precision%29))
  (bind _thirdpersoncharacter (Variables|Default|GetThirdPersonCharacter))
  (bind _thirdpersoncharacter_2 (Variables|Default|GetThirdPersonCharacter))
  (bind _mesh (Variables|Character|GetMesh))
  (bind _returnvalue (Transformation|GetActorLocation _thirdpersoncharacter))
  (bind _returnvalue_2 (Transformation|GetWorldTransform _mesh))
  (bind (_x _y) (Math|Vector|BreakVector _returnvalue))
  (bind _location (Math|Transform|BreakTransform _returnvalue_2))
  (bind (_x_2 _y_2) (Math|Vector|BreakVector _location))
  (if (Variables|Default|GetOverlappingCharacter)
    (Transformation|SetActorRotation (Math|Rotator|FindLookatRotation (Math|Vector|MakeVector _x_2 _y_2 0.0) (Math|Vector|MakeVector _x _y 0.0)))
    (Transformation|SetActorLocation (.Location (Math|Transform|BreakTransform (Math|Transform|Lerp(Transform) (Math|Conversions|ToTransform(Vector) (Transformation|GetActorLocation)) (Math|Conversions|ToTransform(Vector) (Transformation|GetActorLocation _thirdpersoncharacter_2)) (* DeltaSeconds (Variables|Default|GetMoveTimer))))) false false)
    (bind _output_get (Variables|Default|SetNewVar_0 (- (Transformation|GetDistanceTo _thirdpersoncharacter_2) 1.3e+02)))
    (if (<= _output_get 1e+01)
      (bind _asscene_manager (Utilities|Casting|CastToSceneManager (Variables|Default|GetSceneManager)))
      (Variables|/Game/TreasureHunter/Blueprints/SceneManager.SceneManager_C|SetLoseHPString _asscene_manager "SpearIslander")
      (Default|LostHP _asscene_manager)
      (Audio|PlaySoundatLocation "/Game/TreasureHunter/Audio/dying_groan.dying_groan" "0, 0, 0")
      (Effects|SpawnEmitteratLocation "/Game/StarterContent/Particles/P_Explosion.P_Explosion" "0, 0, 0")
      (Actor|DestroyActor))))

(event EventBeginPlay
  (bind _asthird_person_character (Utilities|Casting|CastToThirdPersonCharacter (Game|GetPlayerCharacter 0)))
  (Utilities|Casting|CastToSceneManager (Variables|/Game/ThirdPersonBP/Blueprints/ThirdPersonCharacter.ThirdPersonCharacter_C|GetSceneManager _asthird_person_character))
  (Variables|Default|SetSceneManager (Variables|/Game/ThirdPersonBP/Blueprints/ThirdPersonCharacter.ThirdPersonCharacter_C|GetSceneManager _asthird_person_character))
  (Components|Animation|PlayAnimation (Variables|Character|GetMesh) "/Game/Character/MaleIslander1/Animations/ThirdPersonIdle.ThirdPersonIdle" true))

(fn ConstructionScript)