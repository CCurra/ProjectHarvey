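; Checkpoint actor for the TreasureHunter game that registers itself with the SceneManager while the player stands in it.
; On player overlap, if not already saved, it sets itself as the manager's checkpoint location and flags OnCheckpoint.
; Leaving clears that flag under the same condition.
; A disconnected prompt mentions pressing K to spend a key on saving; the save itself is not handled here.
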(event Collision|EventActorBeginOverlap
  (params (OtherActor :type Actor%20Object%20Reference))
  (if (== OtherActor (Game|GetPlayerCharacter 0))
    (if (not (Variables|Default|GetCheckpointSaved))
      (bind _asscene_manager (Utilities|Casting|CastToSceneManager (Variables|Default|GetSceneManager)))
      (Variables|/Game/TreasureHunter/Blueprints/SceneManager.SceneManager_C|SetCheckpointLoc _asscene_manager self)
      (Variables|/Game/TreasureHunter/Blueprints/SceneManager.SceneManager_C|SetOnCheckpoint _asscene_manager true))))

(event Collision|EventActorEndOverlap
  (params (OtherActor :type Actor%20Object%20Reference))
  (if (== OtherActor (Game|GetPlayerCharacter 0))
    (if (not (Variables|Default|GetCheckpointSaved))
      (bind _asscene_manager (Utilities|Casting|CastToSceneManager (Variables|Default|GetSceneManager)))
      (Variables|/Game/TreasureHunter/Blueprints/SceneManager.SceneManager_C|SetOnCheckpoint _asscene_manager false))))

(fn ConstructionScript)