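; Test climbing actor that moves the third-person character vertically while Q (up) or E (down) is held.
; Key presses store direction and the character's starting Z; while OnClimable is true, Tick steps Z by DeltaSeconds times TimerCount via unswept SetActorLocation.
; Tick also sets IsClimbing on the animation Blueprint to stop the looping jump.
; Nothing here sets OnClimable, and the logic clearing IsClimbing is unconnected.
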(event EventTick
  (params (DeltaSeconds :type Float%20%28single-precision%29))
  (bind _timercount (Variables|Default|GetTimerCount))
  (bind _returnvalue (* DeltaSeconds _timercount))
  ;[1 1 1] EventTick runs every frame. Find if there is a button pressed. If there is cast to the third person and animation blueprints. Then set the climbing variable in the animation Blueprint to true to strop the looping jump. Then use the UpDown bool to set the increment for moving. Then set the actor to that location. Time multiplier at the begining helps move the character over time.
  (if (Variables|Default|GetButtonPressed)
    (if (Variables|Default|GetOnClimable)
      (bind _asthird_person_character (Utilities|Casting|CastToThirdPersonCharacter (Variables|Default|GetThirdPersonCharacter)))
      (bind _asthird_person_anim_bp (Utilities|Casting|CastToThirdPerson_AnimBP (Components|SkeletalMesh|GetAnimInstance (Variables|/Script/Engine.Character|GetMesh (Game|GetPlayerCharacter 0)))))
      (Variables|/Game/Mannequin/Animations/ThirdPerson_AnimBP.ThirdPerson_AnimBP_C|SetIsClimbing _asthird_person_anim_bp true)
      (if (Variables|Default|GetUpDownBool)
        (bind _output_get (Variables|Default|SetGetz (+ (Variables|Default|GetGetz) _returnvalue)))
        (Transformation|SetActorLocation _asthird_person_character (Math|Vector|MakeVector (.X (Math|Vector|BreakVector (Transformation|GetActorLocation _asthird_person_character))) (.Y (Math|Vector|BreakVector (Transformation|GetActorLocation _asthird_person_character))) _output_get) false false)
        (else
          (bind _output_get_2 (Variables|Default|SetGetz (- (Variables|Default|GetGetz) _returnvalue)))
          (Transformation|SetActorLocation _asthird_person_character (Math|Vector|MakeVector (.X (Math|Vector|BreakVector (Transformation|GetActorLocation _asthird_person_character))) (.Y (Math|Vector|BreakVector (Transformation|GetActorLocation _asthird_person_character))) _output_get_2) false false))))))

(event EventBeginPlay
  ;[1 1 1] Enables input for keys
  (Input|EnableInput (Game|GetPlayerController 0)))

(event Input|KeyboardEvents|Q
  (params (Key :type Key%20Structure :default "AnyKey"))
  ;[1 1 1] If Q or E is pressed, set UpDownBool true or false and button pressed. Cast to character to gain the start Z location.
  (:Pressed
    (Variables|Default|SetUpDownBool true)
    (Variables|Default|SetButtonPressed true)
    (bind _asthird_person_character (Utilities|Casting|CastToThirdPersonCharacter (Variables|Default|GetThirdPersonCharacter)))
    (Variables|Default|SetGetz (.Z (Math|Vector|BreakVector (Transformation|GetActorLocation _asthird_person_character)))))
  (:Released
    (Variables|Default|SetButtonPressed false)))

(event Input|KeyboardEvents|E
  (params (Key :type Key%20Structure :default "AnyKey"))
  ;[1 1 1] If Q or E is pressed, set UpDownBool true or false and button pressed. Cast to character to gain the start Z location.
  (:Pressed
    (Variables|Default|SetUpDownBool false)
    (Variables|Default|SetButtonPressed true)
    (bind _asthird_person_character (Utilities|Casting|CastToThirdPersonCharacter (Variables|Default|GetThirdPersonCharacter)))
    (Variables|Default|SetGetz (.Z (Math|Vector|BreakVector (Transformation|GetActorLocation _asthird_person_character)))))
  (:Released
    (Variables|Default|SetButtonPressed false)))

(fn ConstructionScript)