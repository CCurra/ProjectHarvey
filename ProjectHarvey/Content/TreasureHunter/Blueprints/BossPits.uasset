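; BossPits is a boss arena pit trap whose floor drops away when activated.
; On BeginPlay it reaches the EnemyBoss through the player character's SceneManager and registers itself in one of five pit slots chosen by PitNumber.
; Tick polls the Activated flag, then toggles visibility and disables collision on both floor pieces and clears the flag.
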(event EventBeginPlay
  (bind _self self)
  (bind _output_get (Variables|Default|SetThirdPersonCharacter (Game|GetPlayerCharacter 0)))
  (bind _asthird_person_character (Utilities|Casting|CastToThirdPersonCharacter _output_get))
  (bind _output_get_2 (Variables|Default|SetSceneManager (Variables|/Game/ThirdPersonBP/Blueprints/ThirdPersonCharacter.ThirdPersonCharacter_C|GetSceneManager _asthird_person_character)))
  (bind _asscene_manager (Utilities|Casting|CastToSceneManager _output_get_2))
  (bind _output_get_3 (Variables|Default|SetBossMan (Variables|/Game/TreasureHunter/Blueprints/SceneManager.SceneManager_C|GetBossMan _asscene_manager)))
  (bind _asenemy_boss (Utilities|Casting|CastToEnemyBoss _output_get_3))
  (switch int (Variables|Default|GetPitNumber)
    (:1
      (Variables|/Game/TreasureHunter/Blueprints/EnemyBoss.EnemyBoss_C|SetPit1 _asenemy_boss _self))
    (:2
      (Variables|/Game/TreasureHunter/Blueprints/EnemyBoss.EnemyBoss_C|SetPit2 _asenemy_boss _self))
    (:3
      (Variables|/Game/TreasureHunter/Blueprints/EnemyBoss.EnemyBoss_C|SetPit3 _asenemy_boss _self))
    (:4
      (Variables|/Game/TreasureHunter/Blueprints/EnemyBoss.EnemyBoss_C|SetPit4 _asenemy_boss _self))
    (:5
      (Variables|/Game/TreasureHunter/Blueprints/EnemyBoss.EnemyBoss_C|SetPit5 _asenemy_boss _self))))

(event Collision|EventActorBeginOverlap
  (params (OtherActor :type Actor%20Object%20Reference)))

(event EventTick
  (params (DeltaSeconds :type Float%20%28single-precision%29))
  (bind _floor1 (Variables|Default|GetFloor1))
  (if (Variables|Default|GetActivated)
    (Rendering|ToggleVisibility _floor1 false)
    (Collision|SetCollisionEnabled _floor1 "NoCollision")
    (Variables|Default|SetActivated false)))

(fn ConstructionScript)