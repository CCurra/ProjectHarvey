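; Enemy actor for TreasureHunter that chases the player character and costs HP on contact.
; Overlap events toggle a chase flag and print debug messages.
; While the flag is set, Tick yaws the actor toward the player and lerps its location toward them.
; Within a close distance, it passes a SpearIslander damage label to the SceneManager, triggers LostHP and destroys itself.
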(event Collision|EventActorBeginOverlap
  (params (OtherActor :type Actor%20Object%20Reference))
  (if (== OtherActor (Variables|Default|GetThirdPersonCharacter))
    (Variables|Default|SetOverlappingCharacter true)
    (Development|PrintString "Hello")))

(event Collision|EventActorEndOverlap
  (params (OtherActor :type Actor%20Object%20Reference))
  (if (== OtherActor (Variables|Default|GetThirdPersonCharacter))
    (Variables|Default|SetOverlappingCharacter false)
    (Development|PrintString "Bye")))

(event EventTick
  (params (DeltaSeconds :type Float%20%28single-precision%29))
  (bind _thirdpersoncharacter (Variables|Default|GetThirdPersonCharacter))
  (bind _thirdpersoncharacter_2 (Variables|Default|GetThirdPersonCharacter))
  (bind _mesh (Variables|Character|GetMesh))
  (bind _returnvalue (Transformation|GetActorLocation _thirdpersoncharacter))
  (bind _returnvalue_2 (Transformation|GetWorldTransform _mesh))
  (bind (_x _y) (Math|Vector|BreakVector _returnvalue))
  (bind _location (Math|Transform|BreakTransform _returnvalue_2))
  (bind (_x_2 _y_2) (Math|Vector|BreakVector _location))
  (if (Variables|Default|GetOverlappingCharacter)
    (Transformation|SetActorRotation (Math|Rotator|FindLookatRotation (Math|Vector|MakeVector _x_2 _y_2 0.0) (Math|Vector|MakeVector _x _y 0.0)))
    (Transformation|SetActorLocation (.Location (Math|Transform|BreakTransform (Math|Transform|Lerp(Transform) (Math|Conversions|ToTransform(Vector) (Transformation|GetActorLocation)) (Math|Conversions|ToTransform(Vector) (Transformation|GetActorLocation _thirdpersoncharacter_2)) (* DeltaSeconds (Variables|Default|GetMoveTimer))))) false false)
    (bind _output_get (Variables|Default|SetNewVar_0 (- (Transformation|GetDistanceTo _thirdpersoncharacter_2) 1.3e+02)))
    (if (<= _output_get 1e+01)
      (bind _asscene_manager (Utilities|Casting|CastToSceneManager (Variables|Default|GetSceneManager)))
      (Variables|/Game/TreasureHunter/Blueprints/SceneManager.SceneManager_C|SetLoseHPString _asscene_manager "SpearIslander")
      (Default|LostHP _asscene_manager)
      (Actor|DestroyActor))))

(fn ConstructionScript)