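; Spear projectile that costs the player HP on hit, reported to the SceneManager as a "SpearIslander" loss.
; BeginPlay caches the Cube component's world transform as the flight target, toggles the Cube's visibility and enables Capsule collision.
; Tick polls for ThirdPersonCharacter overlaps to trigger LostHP and destroy the spear.
; Otherwise it lerps toward the target by DeltaSeconds times Speed, self-destructing after a frame-time-scaled Delay.
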(event EventBeginPlay
  (bind _asthird_person_character (Utilities|Casting|CastToThirdPersonCharacter (Game|GetPlayerCharacter 0)))
  (Variables|Default|SetNewLocation (Transformation|GetWorldTransform (Variables|Default|GetCube)))
  (Collision|SetCollisionEnabled (Variables|Default|GetCapsule) "QueryAndPhysics")
  (Rendering|ToggleVisibility (Variables|Default|GetCube) false))

(event Collision|EventActorBeginOverlap
  (params (OtherActor :type Actor%20Object%20Reference)))

(event EventTick
  (params (DeltaSeconds :type Float%20%28single-precision%29))
  (if (> (Utilities|Array|Length (Collision|GetOverlappingActors "/Game/ThirdPersonBP/Blueprints/ThirdPersonCharacter.ThirdPersonCharacter_C" :!class /Script/Engine.Actor)) 0)
    (bind _asscene_manager (Utilities|Casting|CastToSceneManager (Variables|/Game/ThirdPersonBP/Blueprints/ThirdPersonCharacter.ThirdPersonCharacter_C|GetSceneManager (stale EventBeginPlay _asthird_person_character))))
    (Variables|/Game/TreasureHunter/Blueprints/SceneManager.SceneManager_C|SetLoseHPString _asscene_manager "SpearIslander")
    (Default|LostHP _asscene_manager)
    (Actor|DestroyActor)
    (else
      (Transformation|SetActorLocation (.Location (Math|Transform|BreakTransform (Math|Transform|Lerp(Transform) (Transformation|GetActorTransform self) (Variables|Default|GetNewLocation) (* DeltaSeconds (Variables|Default|GetSpeed))))) false false)
      (Utilities|FlowControl|Delay (* (Variables|Default|GetDelay) DeltaSeconds))
      (Actor|DestroyActor))))

(fn ConstructionScript)