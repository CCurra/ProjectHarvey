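; Standalone torch actor for TreasureHunter that attaches a particle effect, presumably fire, to actors that overlap it.
; Begin overlap sets an OnFire flag and adds the particle component to the other actor if the flag was clear.
; While OnFire is set, a Delay on Tick adds another component to that actor about every four seconds.
; End overlap clears the flag but removes no particles.
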(event Collision|EventActorBeginOverlap
  (params (OtherActor :type Actor%20Object%20Reference))
  (if (not (Variables|Default|Geton%20fire))
    (Variables|Default|Seton%20fire true)
    (AddComponent|AddParticleSystemComponent OtherActor false)))

(event Collision|EventActorEndOverlap
  (params (OtherActor :type Actor%20Object%20Reference))
  (Variables|Default|Seton%20fire false))

(event EventTick
  (params (DeltaSeconds :type Float%20%28single-precision%29))
  (if (Variables|Default|Geton%20fire)
    (Utilities|FlowControl|Delay 4.0)
    (AddComponent|AddParticleSystemComponent (stale Collision|EventActorBeginOverlap OtherActor) false)))

(fn ConstructionScript)