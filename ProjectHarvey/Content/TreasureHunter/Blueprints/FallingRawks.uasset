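; Falling-rocks trap in the TreasureHunter game that triggers once, when the player character overlaps it.
; The overlap disables the box collision, toggles visibility and enables physics on eleven rock meshes, plays a crumbling sound and calls LostHP on the SceneManager.
; Hit events on ten of the meshes play an impact sound and add a particle component to the struck actor.
; The trap destroys itself after FallDuration.
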(event OnComponentHit(StaticMesh10)
  (params (HitComponent :type Primitive%20Component%20Object%20Reference) (OtherActor :type Actor%20Object%20Reference) (OtherComp :type Primitive%20Component%20Object%20Reference) (NormalImpulse :type Vector :default "0, 0, 0") (Hit :type Hit%20Result%20Structure%20%28by%20ref%29))
  (Audio|SpawnSound2D "/Game/TreasureHunter/Audio/Jab-SoundBible_com-1806727891.Jab-SoundBible_com-1806727891")
  (AddComponent|AddParticleSystemComponent OtherActor false))

(event OnComponentHit(StaticMesh1)
  (params (HitComponent :type Primitive%20Component%20Object%20Reference) (OtherActor :type Actor%20Object%20Reference) (OtherComp :type Primitive%20Component%20Object%20Reference) (NormalImpulse :type Vector :default "0, 0, 0") (Hit :type Hit%20Result%20Structure%20%28by%20ref%29))
  (Audio|SpawnSound2D "/Game/TreasureHunter/Audio/Jab-SoundBible_com-1806727891.Jab-SoundBible_com-1806727891")
  (AddComponent|AddParticleSystemComponent OtherActor false))

(event OnComponentHit(StaticMesh)
  (params (HitComponent :type Primitive%20Component%20Object%20Reference) (OtherActor :type Actor%20Object%20Reference) (OtherComp :type Primitive%20Component%20Object%20Reference) (NormalImpulse :type Vector :default "0, 0, 0") (Hit :type Hit%20Result%20Structure%20%28by%20ref%29))
  (Audio|SpawnSound2D "/Game/TreasureHunter/Audio/Jab-SoundBible_com-1806727891.Jab-SoundBible_com-1806727891")
  (AddComponent|AddParticleSystemComponent OtherActor false))

(event OnComponentHit(StaticMesh2)
  (params (HitComponent :type Primitive%20Component%20Object%20Reference) (OtherActor :type Actor%20Object%20Reference) (OtherComp :type Primitive%20Component%20Object%20Reference) (NormalImpulse :type Vector :default "0, 0, 0") (Hit :type Hit%20Result%20Structure%20%28by%20ref%29))
  (Audio|SpawnSound2D "/Game/TreasureHunter/Audio/Jab-SoundBible_com-1806727891.Jab-SoundBible_com-1806727891")
  (AddComponent|AddParticleSystemComponent OtherActor false))

(event OnComponentHit(StaticMesh3)
  (params (HitComponent :type Primitive%20Component%20Object%20Reference) (OtherActor :type Actor%20Object%20Reference) (OtherComp :type Primitive%20Component%20Object%20Reference) (NormalImpulse :type Vector :default "0, 0, 0") (Hit :type Hit%20Result%20Structure%20%28by%20ref%29))
  (Audio|SpawnSound2D "/Game/TreasureHunter/Audio/Jab-SoundBible_com-1806727891.Jab-SoundBible_com-1806727891")
  (AddComponent|AddParticleSystemComponent OtherActor false))

(event OnComponentHit(StaticMesh7)
  (params (HitComponent :type Primitive%20Component%20Object%20Reference) (OtherActor :type Actor%20Object%20Reference) (OtherComp :type Primitive%20Component%20Object%20Reference) (NormalImpulse :type Vector :default "0, 0, 0") (Hit :type Hit%20Result%20Structure%20%28by%20ref%29))
  (Audio|SpawnSound2D "/Game/TreasureHunter/Audio/Jab-SoundBible_com-1806727891.Jab-SoundBible_com-1806727891")
  (AddComponent|AddParticleSystemComponent OtherActor false))

(event OnComponentHit(StaticMesh5)
  (params (HitComponent :type Primitive%20Component%20Object%20Reference) (OtherActor :type Actor%20Object%20Reference) (OtherComp :type Primitive%20Component%20Object%20Reference) (NormalImpulse :type Vector :default "0, 0, 0") (Hit :type Hit%20Result%20Structure%20%28by%20ref%29))
  (Audio|SpawnSound2D "/Game/TreasureHunter/Audio/Jab-SoundBible_com-1806727891.Jab-SoundBible_com-1806727891")
  (AddComponent|AddParticleSystemComponent OtherActor false))

(event OnComponentHit(StaticMesh6)
  (params (HitComponent :type Primitive%20Component%20Object%20Reference) (OtherActor :type Actor%20Object%20Reference) (OtherComp :type Primitive%20Component%20Object%20Reference) (NormalImpulse :type Vector :default "0, 0, 0") (Hit :type Hit%20Result%20Structure%20%28by%20ref%29))
  (Audio|SpawnSound2D "/Game/TreasureHunter/Audio/Jab-SoundBible_com-1806727891.Jab-SoundBible_com-1806727891")
  (AddComponent|AddParticleSystemComponent OtherActor false))

(event OnComponentHit(StaticMesh4)
  (params (HitComponent :type Primitive%20Component%20Object%20Reference) (OtherActor :type Actor%20Object%20Reference) (OtherComp :type Primitive%20Component%20Object%20Reference) (NormalImpulse :type Vector :default "0, 0, 0") (Hit :type Hit%20Result%20Structure%20%28by%20ref%29))
  (Audio|SpawnSound2D "/Game/TreasureHunter/Audio/Jab-SoundBible_com-1806727891.Jab-SoundBible_com-1806727891")
  (AddComponent|AddParticleSystemComponent OtherActor false))

(event OnComponentHit(StaticMesh9)
  (params (HitComponent :type Primitive%20Component%20Object%20Reference) (OtherActor :type Actor%20Object%20Reference) (OtherComp :type Primitive%20Component%20Object%20Reference) (NormalImpulse :type Vector :default "0, 0, 0") (Hit :type Hit%20Result%20Structure%20%28by%20ref%29))
  (Audio|SpawnSound2D "/Game/TreasureHunter/Audio/Jab-SoundBible_com-1806727891.Jab-SoundBible_com-1806727891")
  (AddComponent|AddParticleSystemComponent OtherActor false))

(event Collision|EventActorBeginOverlap
  (params (OtherActor :type Actor%20Object%20Reference))
  (bind _staticmesh5 (Variables|Default|GetStaticMesh5))
  (if (== OtherActor (Game|GetPlayerCharacter 0))
    (if (not (Variables|Default|GetFalseBool))
      (Variables|Default|SetFalseBool true)
      (Collision|SetCollisionEnabled (Variables|Default|GetBox) "NoCollision")
      (Rendering|ToggleVisibility _staticmesh5 false)
      (Physics|SetSimulatePhysics _staticmesh5 true)
      (Audio|PlaySoundatLocation "/Game/TreasureHunter/Audio/crumbling3.crumbling3" "0, 0, 0")
      (bind _asscene_manager (Utilities|Casting|CastToSceneManager (Variables|Default|GetSceneManager)))
      (Variables|/Game/TreasureHunter/Blueprints/SceneManager.SceneManager_C|SetLoseHPString _asscene_manager "")
      (Default|LostHP _asscene_manager)
      (Utilities|FlowControl|Delay (Variables|Default|GetFallDuration))
      (Actor|DestroyActor))))

(fn ConstructionScript)