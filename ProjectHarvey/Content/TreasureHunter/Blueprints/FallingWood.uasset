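; FallingWood is a pit trap actor in TreasureHunter that collapses and costs HP when something overlaps it.
; The overlap, unfiltered by actor type, disables the Box collision and turns on physics for four wood pieces.
; It then casts its SceneManager reference, reports the HP loss with a "Pit" cause, and destroys itself after FallDuration.
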(event Collision|EventActorBeginOverlap
  (params (OtherActor :type Actor%20Object%20Reference))
  (Collision|SetCollisionEnabled (Variables|Default|GetBox) "NoCollision")
  (Physics|SetSimulatePhysics (Variables|Default|GetWood1) true)
  (bind _asscene_manager (Utilities|Casting|CastToSceneManager (Variables|Default|GetSceneManager)))
  (Variables|/Game/TreasureHunter/Blueprints/SceneManager.SceneManager_C|SetLoseHPString _asscene_manager "Pit")
  (Default|LostHP _asscene_manager)
  (Utilities|FlowControl|Delay (Variables|Default|GetFallDuration))
  (Actor|DestroyActor))

(fn ConstructionScript)