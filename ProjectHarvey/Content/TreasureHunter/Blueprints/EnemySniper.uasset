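; EnemySniper is a stationary enemy that turns toward the player and throws spears once the player enters its overlap area.
; Tick applies a yaw-only look-at, then a Delay scaled by frame time and MoveTimer paces SpearBP spawns below the mesh with a whoosh sound.
; End overlap compares against the PlayerController instead of the character, so tracking never switches off.
; BeginPlay caches the player's SceneManager and toggles Cube1's visibility.
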(event Collision|EventActorBeginOverlap
  (params (OtherActor :type Actor%20Object%20Reference))
  (bind _returnvalue (Game|GetPlayerCharacter 0))
  (if (== OtherActor _returnvalue)
    (Variables|Default|SetThirdPersonCharacter _returnvalue)
    (Variables|Default|SetOverlappingCharacter true)
    (Development|PrintString "Hello")))

(event Collision|EventActorEndOverlap
  (params (OtherActor :type Actor%20Object%20Reference))
  (if (== OtherActor (Game|GetPlayerController 0))
    (Variables|Default|SetOverlappingCharacter false)
    (Development|PrintString "Bye")))

(event EventTick
  (params (DeltaSeconds :type Float%20%28single-precision%29))
  (bind _mesh (Variables|Character|GetMesh))
  (bind _thirdpersoncharacter (Variables|Default|GetThirdPersonCharacter))
  (bind _mesh_2 (Variables|Character|GetMesh))
  (bind _returnvalue (Transformation|GetActorLocation _thirdpersoncharacter))
  (bind _returnvalue_2 (Transformation|GetWorldTransform _mesh_2))
  (bind _returnvalue_3 (Transformation|GetWorldTransform _mesh))
  (bind (_x _y) (Math|Vector|BreakVector _returnvalue))
  (bind _location (Math|Transform|BreakTransform _returnvalue_2))
  (bind (_location_2 _rotation) (Math|Transform|BreakTransform _returnvalue_3))
  (bind (_x_2 _y_2 _z) (Math|Vector|BreakVector _location_2))
  (bind (_x_3 _y_3) (Math|Vector|BreakVector _location))
  (if (Variables|Default|GetOverlappingCharacter)
    (Transformation|SetActorRotation (Math|Rotator|FindLookatRotation (Math|Vector|MakeVector _x_3 _y_3 0.0) (Math|Vector|MakeVector _x _y 0.0)))
    (Utilities|FlowControl|Delay (* DeltaSeconds (Variables|Default|GetMoveTimer)))
    (Game|SpawnActorfromClass "/Game/TreasureHunter/Blueprints/SpearBP.SpearBP_C" (Math|Transform|MakeTransform (Math|Vector|MakeVector _x_2 _y_2 (- _z 8e+01)) _rotation "0.200000,0.200000,0.200000") "Undefined" 0 0)
    (Audio|PlaySound2D "/Game/TreasureHunter/Audio/Woosh-Mark_DiAngelo-4778593.Woosh-Mark_DiAngelo-4778593")))

(event EventBeginPlay
  (bind _asthird_person_character (Utilities|Casting|CastToThirdPersonCharacter (Game|GetPlayerCharacter 0)))
  (Utilities|Casting|CastToSceneManager (Variables|/Game/ThirdPersonBP/Blueprints/ThirdPersonCharacter.ThirdPersonCharacter_C|GetSceneManager _asthird_person_character))
  (Variables|Default|SetSceneManager (Variables|/Game/ThirdPersonBP/Blueprints/ThirdPersonCharacter.ThirdPersonCharacter_C|GetSceneManager _asthird_person_character))
  (Rendering|ToggleVisibility (Variables|Default|GetCube1) false))

(fn ConstructionScript)