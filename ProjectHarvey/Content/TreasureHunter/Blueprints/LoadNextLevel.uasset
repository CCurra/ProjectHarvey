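; LoadNextLevel is a trigger actor that lets the player travel to another level with an input action.
; When the player's ThirdPersonCharacter overlaps the Box, it sets a Trigger flag, which is never cleared, and casts SceneManager without using the result.
; The actor enables input on BeginPlay, and pressing NextLevel opens TargetLevel by name once the flag is set.
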(event OnComponentBeginOverlap(Box)
  (params (OverlappedComponent :type Primitive%20Component%20Object%20Reference) (OtherActor :type Actor%20Object%20Reference) (OtherComp :type Primitive%20Component%20Object%20Reference) (OtherBodyIndex :type Integer) (bFromSweep :type Boolean) (SweepResult :type Hit%20Result%20Structure%20%28by%20ref%29))
  (bind _asthird_person_character (Utilities|Casting|CastToThirdPersonCharacter OtherActor))
  (if (== _asthird_person_character (Game|GetPlayerCharacter 0))
    (Variables|Default|SetTrigger true)
    (Utilities|Casting|CastToSceneManager (Variables|Default|Getscene%20manager))))

(event Collision|EventActorBeginOverlap
  (params (OtherActor :type Actor%20Object%20Reference)))

(event EventBeginPlay
  (Input|EnableInput (Game|GetPlayerController 0)))

(event Input|ActionEvents|InputActionNextLevel
  (params (Key :type Key%20Structure :default "AnyKey"))
  (:Pressed
    (if (Variables|Default|GetTrigger)
      (Game|OpenLevel(byName) (Variables|Default|GetTargetLevel)))))

(fn ConstructionScript)