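; Actor Blueprint that opens the pause menu when P is pressed, after enabling player-one input on BeginPlay.
; The key press creates a Pause_Menu_Widget, adds it to the viewport, switches to UI-only input with the cursor shown, and pauses the game.
; The validity check before creation has no input and the widget reference assignment is disconnected, so the widget is never cached.
; Nothing here resumes the game.
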(event EventBeginPlay
  (Input|EnableInput (Game|GetPlayerController 0)))

(event Input|KeyboardEvents|P
  (params (Key :type Key%20Structure :default "AnyKey"))
  (bind _returnvalue (Game|GetPlayerController 0))
  (:Pressed
    (Utilities|IsValid 0
      (:Is%20Valid
        _)
      (:Is%20Not%20Valid
        (bind _returnvalue_2 (UserInterface|CreateWidget "/Game/TreasureHunter/Blueprints/Pause_Menu_Widget.Pause_Menu_Widget_C"))))
    (Input|SetInputModeUIOnly _returnvalue 0 "DoNotLock")
    (UserInterface|Viewport|AddtoViewport _returnvalue_2 0)
    (Variables|/Script/Engine.PlayerController|SetbShowMouseCursor _returnvalue true)
    (Game|SetGamePaused true)))

(fn ConstructionScript)