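; Quicksand actor that sinks while the player's ThirdPersonCharacter stands in it.
; Each Tick, any character overlapping the Box moves the whole actor down by a fixed step, so sink speed depends on frame rate.
; A character hit on OtherFrigginCube snaps the actor's height to a fixed offset below that character, keeping X and Y.
; An alternative height-snapping branch is left unconnected and never runs.
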(event OnComponentHit(otherfriggincube)
  (params (HitComponent :type Primitive%20Component%20Object%20Reference) (OtherActor :type Actor%20Object%20Reference) (OtherComp :type Primitive%20Component%20Object%20Reference) (NormalImpulse :type Vector :default "0, 0, 0") (Hit :type Hit%20Result%20Structure%20%28by%20ref%29))
  (bind _returnvalue (Transformation|GetActorLocation))
  (bind (_x _y _z) (Math|Vector|BreakVector _returnvalue))
  (bind _asthird_person_character (Utilities|Casting|CastToThirdPersonCharacter OtherActor))
  (Transformation|SetActorLocation (Math|Vector|MakeVector _x _y (- (.Z (Math|Vector|BreakVector (Transformation|GetActorLocation _asthird_person_character))) 96.0)) false false))

(event EventBeginPlay)

(event Collision|EventActorBeginOverlap
  (params (OtherActor :type Actor%20Object%20Reference)))

(event EventTick
  (params (DeltaSeconds :type Float%20%28single-precision%29))
  (bind _returnvalue (Transformation|GetActorLocation))
  (bind (_x _y _z) (Math|Vector|BreakVector _returnvalue))
  (if (> (Utilities|Array|Length (Collision|GetOverlappingActors (Variables|Default|GetBox) "/Game/ThirdPersonBP/Blueprints/ThirdPersonCharacter.ThirdPersonCharacter_C" :!class /Script/Engine.PrimitiveComponent)) 0)
    (Transformation|SetActorLocation (Math|Vector|MakeVector _x _y (+ _z -0.5)) false false)))

(fn ConstructionScript)