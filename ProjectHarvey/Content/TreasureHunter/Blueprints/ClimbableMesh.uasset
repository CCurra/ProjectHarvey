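; Climbable actor that flags TempClimbTest as climbable on overlap and holds the player in place between climb inputs.
; Q inside the overlap arms the hold, and releasing Q or E then stores the player controller's location.
; While armed, overlapping and unpressed, Tick pins the character there by setting its location each frame.
; BeginPlay disables Top and Bottom collision; unconnected gravity and animation-reset nodes never run.
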(event Collision|EventActorBeginOverlap
  (params (OtherActor :type Actor%20Object%20Reference))
  (bind _astemp_climb_test (Utilities|Casting|CastToTempClimbTest (Variables|Default|GetClimbScript)))
  (Variables|/Game/TreasureHunter/Blueprints/TempClimbTest.TempClimbTest_C|SetOnClimable _astemp_climb_test true)
  (Variables|Default|SetIsOverlapping true))

(event EventTick
  (params (DeltaSeconds :type Float%20%28single-precision%29))
  (Input|EnableInput (Game|GetPlayerController 0))
  (if (Variables|Default|GetIsOverlapping)
    (if (not (Variables|Default|GetButtonPressed))
      (if (Variables|Default|GetFirstButtonPressed)
        (Transformation|SetActorLocation (Game|GetPlayerCharacter 0) (Variables|Default|GetGetStop) false false)))))

(event Collision|EventActorEndOverlap
  (params (OtherActor :type Actor%20Object%20Reference))
  (bind _astemp_climb_test (Utilities|Casting|CastToTempClimbTest (Variables|Default|GetClimbScript)))
  (Variables|/Game/TreasureHunter/Blueprints/TempClimbTest.TempClimbTest_C|SetOnClimable _astemp_climb_test false)
  (Variables|Default|SetIsOverlapping false)
  (Variables|Default|SetFirstButtonPressed false))

(event EventBeginPlay
  (Collision|SetCollisionEnabled (Variables|Default|GetTop) "NoCollision")
  (Input|EnableInput 0))

(event Input|KeyboardEvents|Q
  (params (Key :type Key%20Structure :default "AnyKey"))
  (:Pressed
    (if (Variables|Default|GetIsOverlapping)
      (Variables|Default|SetFirstButtonPressed true)
      (Variables|Default|SetButtonPressed true)))
  (:Released
    (if (Variables|Default|GetFirstButtonPressed)
      (Variables|Default|SetGetStop (Transformation|GetActorLocation (Game|GetPlayerController 0)))
      (Variables|Default|SetButtonPressed false))))

(event Input|KeyboardEvents|E
  (params (Key :type Key%20Structure :default "AnyKey"))
  (:Pressed
    (Variables|Default|SetButtonPressed true))
  (:Released
    (if (Variables|Default|GetFirstButtonPressed)
      (Variables|Default|SetGetStop (Transformation|GetActorLocation (Game|GetPlayerController 0)))
      (Variables|Default|SetButtonPressed false))))

(fn ConstructionScript)