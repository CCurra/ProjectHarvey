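; SaveManager is an actor that restores a level's Points from a save slot named after LevelName in TreasureHunter.
; On BeginPlay it loads an existing Save into SaveInstance and copies its Points to SceneManager, or creates a new Save tagged with LevelName.
; Saving is unfinished: Tick only casts SceneManager, the Points write-back is disconnected, and nothing writes the slot to disk.
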(event EventBeginPlay
  (bind _returnvalue (SaveGame|DoesSaveGameExist (Utilities|String|ToString(Name) (Variables|Default|GetLevelName))))
  (if _returnvalue
    (bind _returnvalue_2 (SaveGame|LoadGamefromSlot (Utilities|String|ToString(Name) (Variables|Default|GetLevelName))))
    (bind _assave (Utilities|Casting|CastToSave _returnvalue_2))
    (bind _output_get (Variables|Default|SetSaveInstance _assave))
    (bind _asscene_manager (Utilities|Casting|CastToSceneManager (Variables|Default|GetScene%20manager)))
    (Variables|/Game/TreasureHunter/Blueprints/SceneManager.SceneManager_C|SetPoints _asscene_manager (Variables|/Game/TreasureHunter/Blueprints/Save.Save_C|GetPoints _output_get))
    (else
      (bind _returnvalue_3 (SaveGame|CreateSaveGameObject "/Game/TreasureHunter/Blueprints/Save.Save_C"))
      (bind _output_get_2 (Variables|Default|SetSaveInstance _returnvalue_3))
      (Variables|/Game/TreasureHunter/Blueprints/Save.Save_C|SetLevelName _output_get_2 (Variables|Default|GetLevelName)))))

(event Collision|EventActorBeginOverlap
  (params (OtherActor :type Actor%20Object%20Reference)))

(event EventTick
  (params (DeltaSeconds :type Float%20%28single-precision%29))
  (bind _asscene_manager (Utilities|Casting|CastToSceneManager (Variables|Default|GetScene%20manager))))

(fn ConstructionScript)