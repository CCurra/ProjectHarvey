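; Spike trap actor that costs the player health when the player character overlaps it.
; On BeginPlay it caches the SceneManager reference from the ThirdPersonCharacter.
; Player overlap sets the SceneManager's LoseHPString to "RockSmall", the damage key, and calls LostHP once per entry.
; An IsOverlapping flag tracks contact, but nothing repeats the damage while the player stays inside.
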(event Collision|EventActorBeginOverlap
  (params (OtherActor :type Actor%20Object%20Reference))
  (if (== OtherActor (Game|GetPlayerCharacter 0))
    (Variables|Default|SetIsOverlapping true)
    (if (Variables|Default|GetIsOverlapping)
      (bind _asscene_manager (Utilities|Casting|CastToSceneManager (Variables|Default|GetSceneManager)))
      (Variables|/Game/TreasureHunter/Blueprints/SceneManager.SceneManager_C|SetLoseHPString _asscene_manager "RockSmall")
      (Default|LostHP _asscene_manager))))

(event Collision|EventActorEndOverlap
  (params (OtherActor :type Actor%20Object%20Reference))
  (if (== OtherActor (Game|GetPlayerCharacter 0))
    (Variables|Default|SetIsOverlapping false)))

(event EventBeginPlay
  (bind _asthird_person_character (Utilities|Casting|CastToThirdPersonCharacter (Game|GetPlayerCharacter 0)))
  (Variables|Default|SetSceneManager (Variables|/Game/ThirdPersonBP/Blueprints/ThirdPersonCharacter.ThirdPersonCharacter_C|GetSceneManager _asthird_person_character)))

(fn ConstructionScript)