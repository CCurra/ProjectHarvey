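; SceneManager is the player game-state manager for TreasureHunter, handling health, stamina, keys, medkits, checkpoints and game over.
; It creates the HUD and enables input for Shift sprinting, with stamina updated on Tick, and for K, which spends a key to save a checkpoint.
; LostHP maps hazard or med-pack names to health changes, triggering OnDeath, which teleports to the checkpoint or loads EndLevel without decrementing lives.
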(event EventBeginPlay
  ;[1 1 1] Enables Input
  (Variables|Default|SetCharacter (Game|GetPlayerCharacter 0))
  (bind _returnvalue (UserInterface|CreateWidget "/Game/TreasureHunter/ProgrammerLevels/ProgrammerHUD/HUDWidgetP.HUDWidgetP_C"))
  (UserInterface|Viewport|AddtoViewport _returnvalue 0)
  (Input|EnableInput (Game|GetPlayerController 0))
  (bind _asthird_person_character (Utilities|Casting|CastToThirdPersonCharacter (Variables|Default|GetCharacter)))
  (Variables|/Script/Engine.CharacterMovementComponent|SetMaxWalkSpeed (Variables|/Script/Engine.Character|GetCharacterMovement _asthird_person_character) 6e+02)
  (Variables|Default|SetRunFull false))

(event EventTick
  (params (DeltaSeconds :type Float%20%28single-precision%29))
  (if (>= (Variables|Default|GetStamina) 0.0)
    (if (> (Variables|Default|GetStamina) 1e+02)
      (Variables|Default|SetStamina 1e+02)
      (elif (Variables|Default|GetIsRunning)
        (bind _output_get (Variables|Default|SetTimeIncrease (* DeltaSeconds (Variables|Default|GetTimeDecVar))))
        (Variables|Default|SetStamina (- (Variables|Default|GetStamina) _output_get))
        (else
          (bind _output_get_2 (Variables|Default|SetTimeIncrease (* DeltaSeconds (Variables|Default|GetTimeIncVar))))
          (if (< (Variables|Default|GetStamina) 1e+02)
            (if (>= (Variables|Default|GetStamina) 0.0)
              (Variables|Default|SetStamina (+ (Variables|Default|GetStamina) _output_get_2)))))))
    (else
      (Variables|Default|SetStamina 0.0)
      (Variables|Default|SetRunFull true)
      (Variables|Default|SetIsRunning false)
      (bind _asthird_person_character (Utilities|Casting|CastToThirdPersonCharacter (Variables|Default|GetCharacter)))
      (Variables|/Script/Engine.CharacterMovementComponent|SetMaxWalkSpeed (Variables|/Script/Engine.Character|GetCharacterMovement _asthird_person_character) 6e+02))))

(event Input|KeyboardEvents|K
  (params (Key :type Key%20Structure :default "AnyKey"))
  ;[1 1 1] Setting checkpoint system
  (:Pressed
    (if (Variables|Default|GetOnCheckpoint)
      (if (Game|Player|IsInputKeyDown (Game|GetPlayerController 0) (Variables|Default|GetK%20Key))
        (CallFunction|SetCheckpoint)))))

(event Input|KeyboardEvents|L
  (params (Key :type Key%20Structure :default "AnyKey"))
  ;[1 1 1] Debug-Location (Temporary)
  (:Pressed
    (Development|PrintString (Utilities|String|ToString(Vector) (Transformation|GetActorLocation (Variables|Default|GetCharacter))))))

(event Input|KeyboardEvents|LeftShift
  (params (Key :type Key%20Structure :default "AnyKey"))
  (bind _character (Variables|Default|GetCharacter))
  (:Pressed
    (if (Variables|Default|GetRunFull)
      (bind _asthird_person_character (Utilities|Casting|CastToThirdPersonCharacter _character :!label _label))
      (Variables|/Script/Engine.CharacterMovementComponent|SetMaxWalkSpeed (Variables|/Script/Engine.Character|GetCharacterMovement _asthird_person_character) 6e+02)
      (Variables|Default|SetRunFull false)
      (elif (> (Variables|Default|GetStamina) 0.0)
        (Variables|Default|SetIsRunning true)
        (Utilities|Casting|CastToThirdPersonCharacter _character)
        (Variables|/Script/Engine.CharacterMovementComponent|SetMaxWalkSpeed (Variables|/Script/Engine.Character|GetCharacterMovement _asthird_person_character) 9e+02))))
  (:Released
    (Variables|Default|SetIsRunning false)
    (goto _label)))

(fn ConstructionScript)

(fn LostHP
  (switch string (Variables|Default|GetLoseHPString)
    (:RockSmall
      (Variables|Default|SetHealth (- (Variables|Default|GetHealth) (Variables|Default|GetThirdHP)) :!label _label))
    (:RockLarge
      (Variables|Default|SetHealth (- (Variables|Default|GetHealth) (Variables|Default|GetHalfHP))))
    (:SpearIslander
      (goto _label))
    (:SpearBoss
      (Variables|Default|SetHealth (- (Variables|Default|GetHealth) (Variables|Default|GetKoHP)) :!label _label_2))
    (:Pit
      (goto _label_2))
    (:Quicksand
      (goto _label_2))
    (:WallClosing
      (goto _label_2))
    (:MedPack
      (Variables|Default|SetHealth (Variables|Default|GetFullHP))))
  (if (<= (Variables|Default|GetHealth) 0)
    (CallFunction|OnDeath)))

(fn OnDeath
  (if (Variables|Default|GetAnyCheckpointSaved)
    (if (>= (Variables|Default|GetLifes) 1)
      (Transformation|SetActorLocation (Variables|Default|GetCharacter) (Variables|Default|GetCheckpoint) false false)
      (else
        (CallFunction|GameOver :!label _label)))
    (else
      (goto _label))))

(fn FKeyGL
  (switch string (Variables|Default|GetKeyGL)
    (:Gain
      (Variables|Default|SetKeys (+ (Variables|Default|GetKeys) 1)))
    (:Lose
      (Variables|Default|SetKeys (- (Variables|Default|GetKeys) 1)))))

(fn FMedkitGL
  (switch string (Variables|Default|GetMedKitGL)
    (:Gain
      (Variables|Default|SetMedKit (+ (Variables|Default|GetMedKit) 0)))
    (:Lose
      (Variables|Default|SetMedKit (- (Variables|Default|GetMedKit) 1)))))

(fn SetCheckpoint
  (if (>= (Variables|Default|GetKeys) 1)
    (Variables|Default|SetKeys (- (Variables|Default|GetKeys) 1))
    (bind _ascheckpoint_location (Utilities|Casting|CastToCheckpointLocation (Variables|Default|GetCheckpointLoc)))
    (Variables|/Game/TreasureHunter/Blueprints/CheckpointLocation.CheckpointLocation_C|SetCheckpointSaved _ascheckpoint_location true)
    (Variables|Default|SetCheckpoint (Transformation|GetActorLocation (Variables|Default|GetCharacter)))
    (Variables|Default|SetOnCheckpoint false)
    (Development|PrintString "Checkpoint Saved!")
    (Variables|Default|SetAnyCheckpointSaved true)))

(fn GameOver
  (Game|OpenLevel(byName) "EndLevel"))